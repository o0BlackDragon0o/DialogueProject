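; DialogueControllerBP is an actor that sets up and triggers dialogue through its AI controller.
; On BeginPlay it passes its DiagTree to the DiagAIController, then adds a Hud_josh widget to the viewport and registers it with DiagGameMode as the Hud.
; Its StartDialogue event forwards the call to the same controller and prints a debug message.
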(event Custom|Start%20Dialogue
  (bind _asdiag_aicontroller (Utilities|Casting|CastToDiagAIController (AI|GetAIController self)))
  (Default|StartDialogue _asdiag_aicontroller)
  (Development|PrintString "started dialogue!!"))

(event EventBeginPlay
  (bind _asdiag_aicontroller (Utilities|Casting|CastToDiagAIController (AI|GetAIController self)))
  (Variables|/Game/misc/Npc/DiagAIController.DiagAIController_C|SetDaigTree _asdiag_aicontroller (Variables|Default|GetDiagTree))
  (bind _returnvalue (UserInterface|CreateWidget "/Game/UI/Hud_josh.Hud_josh_C" (Game|GetPlayerController 0)))
  (UserInterface|Viewport|AddtoViewport _returnvalue 0)
  (bind _asdiag_game_mode (Utilities|Casting|CastToDiagGameMode (Game|GetGameMode)))
  (Variables|/Game/misc/DiagGameMode.DiagGameMode_C|SetHud _asdiag_game_mode _returnvalue))

(fn ConstructionScript)